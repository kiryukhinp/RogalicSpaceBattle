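; Player-controlled Paper2D ship for a shooter, moving along its forward vector from right-axis input and nudged back along X when out of bounds.
; Held fire spawns twin shots on a looping timer and swaps flipbooks, while StrikeWave spawns on a cooldown, both gated by DoOnce.
; Enemy overlaps reduce health shown on the Overlay widget; death spawns an explosion and switches its panel, which pause also toggles.
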(event `InputAction|StrikeWave`
  (params (Key :type "Key Structure"))
  (:`Pressed`
    (`/Engine/EditorBlueprintResources/StandardMacros.DoOnce` false :!label _label
      (:`Completed`
        (`|SpawnActorFromClass` "/Game/Blueprints/StrikeWave.StrikeWave_C" (`SceneComponent.K2_GetComponentToWorld` (`self.Ship`)) "Undefined" "OverrideRootScale" null null)
        (`KismetSystemLibrary.Delay` 5.0)
        (goto _label :!via `Reset`)))))

(event `self.ReceiveBeginPlay`
  (`SceneComponent.K2_SetWorldLocation` (`self.Ship`) (0.0 0.0 -350.0) false false)
  (set `self.Current _Health` (`self.Full_Health`))
  (bind _foundwidgets (`WidgetBlueprintLibrary.GetAllWidgetsOfClass` "/Game/UI/Overlay.Overlay_C"))
  (set `self.Ovrlay reference` (`|GetArrayItem` _foundwidgets)))

(event `self.ReceiveTick`
  (params (DeltaSeconds :type "Float (single-precision)"))
  (bind _ship (`self.Ship`))
  (bind (_returnvalue_x _returnvalue_y _returnvalue_z) (`KismetMathLibrary.BreakVector` (`SceneComponent.K2_GetComponentLocation` (`self.Ship`))))
  (bind _returnvalue (`KismetMathLibrary.Abs` _returnvalue_x))
  (if (and (<= _returnvalue 600.0) (<= (`KismetMathLibrary.Abs` _returnvalue_z) 400.0))
    (`SceneComponent.K2_AddLocalOffset` _ship (* (+ (0.0 0.0 0.0) (* (`SceneComponent.GetForwardVector` (`self.Ship`)) (* (`self.GetInputAxisValue`) (`self.Max_Sped`)))) DeltaSeconds) false false)
    (else
      (`SceneComponent.K2_AddLocalOffset` _ship (`KismetMathLibrary.MakeVector` (* (/ _returnvalue _returnvalue_x) -1.0)) false false))))

(event `InputAction|Fire`
  (params (Key :type "Key Structure"))
  (:`Pressed`
    (`/Engine/EditorBlueprintResources/StandardMacros.DoOnce` false :!label _label_2
      (:`Completed`
        (`PaperFlipbookComponent.SetFlipbook` (`self.Ship`) "/Game/Sprites/Player_SS/SS_Fire.SS_Fire")
        (`self.OpenFire`)
        (`KismetSystemLibrary.Delay` 0.5)
        (goto _label_2 :!via `Reset`))))
  (:`Released`
    (`PaperFlipbookComponent.SetFlipbook` (`self.Ship`) "/Game/Sprites/Player_SS/Base_SS_anim.Base_SS_anim")
    (`self.StopFire`)))

(event `StopFire`
  (`KismetSystemLibrary.K2_PauseTimerHandle` (stale `OpenFire` _returnvalue)))

(event `OpenFire`
  (`self.Fire`)
  (bind _returnvalue (`KismetSystemLibrary.K2_SetTimer` null "Fire" 0.5 true)))

(event `self.ReceiveActorBeginOverlap`
  (params (OtherActor :type "Actor Object Reference"))
  (bind _ovrlay_reference (`self.Ovrlay reference`))
  (bind _asenemy (cast `/Game/Blueprints/Enemy` OtherActor))
  (set `self.Current _Health` (- (`self.Current _Health`) (`/Game/Blueprints/Enemy.CollideDamage` _asenemy)))
  (`/Game/UI/Overlay.Update Health` (`self.Ovrlay reference`) (`self.Current _Health`) (`self.Full_Health`))
  (if (<= (`self.Current _Health`) 0)
    (set `self.IsGameOver` true)
    (`|SpawnActorFromClass` "/Game/Blueprints/Blow_Up.Blow_Up_C" (`SceneComponent.K2_GetComponentToWorld` (`self.Ship`)) "Undefined" "OverrideRootScale" null null)
    (`WidgetSwitcher.SetActiveWidgetIndex` (`/Game/UI/Overlay.WidgetSwitcher_0` _ovrlay_reference) 1)
    (`TextBlock.SetText` (`/Game/UI/Overlay.TextBlock_120` _ovrlay_reference) (`TextBlock.GetText` (`/Game/UI/Overlay.TextBlock_61` _ovrlay_reference)))
    (`self.K2_DestroyActor`)))

(event `InputAction|Pause` :paused true
  (params (Key :type "Key Structure"))
  (bind _widgetswitcher_0 (`/Game/UI/Overlay.WidgetSwitcher_0` (`self.Ovrlay reference`)))
  (:`Pressed`
    (if (not (`self.IsGameOver`))
      (`/Engine/EditorBlueprintResources/StandardMacros.FlipFlop`
        (:`A`
          (`GameplayStatics.SetGamePaused` true)
          (`WidgetSwitcher.SetActiveWidgetIndex` _widgetswitcher_0 2))
        (:`B`
          (`GameplayStatics.SetGamePaused` false)
          (`WidgetSwitcher.SetActiveWidgetIndex` _widgetswitcher_0 0))))))

(fn `Fire`
  (bind _returnvalue (`SceneComponent.K2_GetComponentToWorld` (`self.Ship`)))
  (bind _returnvalue_2 (`SceneComponent.K2_GetComponentToWorld` (`self.Ship`)))
  (`|SpawnActorFromClass` "/Game/Blueprints/Fire.Fire_C" (`KismetMathLibrary.MakeTransform` (`KismetMathLibrary.MakeVector` (+ (.x (.location _returnvalue_2)) 33.0) (.y (.location _returnvalue_2)) (+ (.z (.location _returnvalue_2)) 50.0)) (struct) (2.0 1.0 2.0)) "Undefined" "OverrideRootScale" null null)
  (`|SpawnActorFromClass` "/Game/Blueprints/Fire.Fire_C" (`KismetMathLibrary.MakeTransform` (`KismetMathLibrary.MakeVector` (+ (.x (.location _returnvalue)) -33.0) (.y (.location _returnvalue)) (+ (.z (.location _returnvalue)) 50.0)) (struct) (2.0 1.0 2.0)) "Undefined" "OverrideRootScale" null null))

(fn `UserConstructionScript`)