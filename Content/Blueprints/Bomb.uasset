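; Bomb for a space game that, when hit, expands and damages space objects and player ships it overlaps.
; OnHit runs the parent logic, then starts a fast looping timer on BlowUp, which grows the actor uniformly each tick and calls Blow at maximum scale.
; Overlaps record each actor in DamagedActors to avoid repeat damage, passing Damage to SpaceObject.OnHit, which can trigger other objects' hit reactions, or to PlayerShip.
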(event `self.ReceiveBeginPlay`
  (`parent.ReceiveBeginPlay`))

(event `self.OnHit`
  (params (Damage :type Integer))
  (`parent.OnHit` Damage)
  (`KismetSystemLibrary.K2_SetTimer` self "BlowUp" 0.01 true))

(event `self.ReceiveActorBeginOverlap`
  (params (OtherActor :type "Actor Object Reference"))
  (bind _damagedactors (`self.DamagedActors`))
  (if (not (`BlueprintSetLibrary.Set_Contains` _damagedactors OtherActor))
    (`BlueprintSetLibrary.Set_Add` _damagedactors OtherActor)
    (bind _asspace_object (cast `/Game/Blueprints/SpaceObject` OtherActor)
      (:`then`
        (`self.OnHit` _asspace_object (`self.Damage`)))
      (:`CastFailed`
        (bind _asplayer_ship (cast `/Game/Blueprints/PlayerShip` OtherActor))
        (`/Game/Blueprints/PlayerShip.AddDmamge` _asplayer_ship (`self.Damage`))))))

(fn `BlowUp`
  (bind (_returnvalue_x _returnvalue_y _returnvalue_z) (`KismetMathLibrary.BreakVector` (`self.GetActorScale3D` self)))
  (if (>= _returnvalue_z (`self.MaxScale`))
    (`self.Blow`)
    (else
      (`self.SetActorRelativeScale3D` (`KismetMathLibrary.Conv_DoubleToVector` (+ _returnvalue_x (`self.StepScale`)))))))

(fn `UserConstructionScript`
  (`parent.UserConstructionScript`))