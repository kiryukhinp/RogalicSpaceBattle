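; Enemy fighter ship that tracks the player's ship along X and fires paired projectiles at a fixed rate.
; Looping timers spawn two offset EnemyFire shots and update the horizontal direction toward the player, which Tick applies through a Gate.
; When a Fire actor overlaps its Box, it dodges toward world X zero by pausing tracking briefly, with a DoOnce blocking repeat dodges until the delay ends.
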(event `self.ReceiveBeginPlay`
  (`parent.ReceiveBeginPlay`)
  (`|ExecutionSequence`
    (:`then_0`
      (bind _asplayer_ship (cast `/Game/Blueprints/PlayerShip` (`GameplayStatics.GetPlayerPawn` 0)))
      (set `self.PlayerShipRef` _asplayer_ship))
    (:`then_1`
      (`KismetSystemLibrary.K2_SetTimer` null "Shoot" (/ 1.0 (`self.FireRate`)) true)
      (bind _returnvalue (`KismetSystemLibrary.K2_SetTimer` null "ChangeLocation" 0.5 true))
      (set `self.ChLocTimerHandle` _returnvalue))))

(event `TryToDodge`
  (bind _returnvalue_x (`KismetMathLibrary.BreakVector` (`self.K2_GetActorLocation`)))
  (bind _returnvalue (`KismetMathLibrary.SignOfFloat` _returnvalue_x))
  (`KismetSystemLibrary.K2_PauseTimerHandle` (`self.ChLocTimerHandle`))
  (if (!= _returnvalue 0.0)
    (set `self.Rule` (* _returnvalue -1.0))
    (goto _label :!via `Open`)
    (else
      (set `self.Rule` -1.0)
      (goto _label :!via `Open`))))

(event `self.ReceiveTick`
  (params (DeltaSeconds :type "Float (single-precision)"))
  (`parent.ReceiveTick` DeltaSeconds)
  (`/Engine/EditorBlueprintResources/StandardMacros.Gate` false :!label _label
    (:`Exit`
      (`self.K2_AddActorLocalOffset` (`KismetMathLibrary.MakeVector` (* DeltaSeconds (`self.XSpeed`) (`self.Rule`)))))))

(event `self.Box.OnComponentBeginOverlap`
  (params (OverlappedComponent :type "PrimitiveComponent Object Reference") (OtherActor :type "Actor Object Reference") (OtherComp :type "PrimitiveComponent Object Reference") (OtherBodyIndex :type Integer) (bFromSweep :type Boolean) (SweepResult :type "HitResult Structure (by ref)"))
  (cast `/Game/Blueprints/Fire` OtherActor)
  (`/Engine/EditorBlueprintResources/StandardMacros.DoOnce` false :!label _label_2
    (:`Completed`
      (`self.TryToDodge`)
      (`KismetSystemLibrary.Delay` 0.5)
      (`|ExecutionSequence`
        (:`then_1`
          (`KismetSystemLibrary.K2_UnPauseTimerHandle` (`self.ChLocTimerHandle`)))
        (:`then_2`
          (goto _label_2 :!via `Reset`))))))

(fn `ChangeLocation`
  (bind _returnvalue_x (`KismetMathLibrary.BreakVector` (`self.K2_GetActorLocation`)))
  (bind _returnvalue_x_2 (`KismetMathLibrary.BreakVector` (`SceneComponent.K2_GetComponentLocation` (`/Game/Blueprints/PlayerShip.Box` (`self.PlayerShipRef`)))))
  (set `self.Rule` (`KismetMathLibrary.SignOfFloat` (- _returnvalue_x_2 _returnvalue_x))))

(fn `Shoot`
  (bind _returnvalue (`SceneComponent.K2_GetComponentToWorld` (`self.Base`)))
  (bind _returnvalue_2 (`SceneComponent.K2_GetComponentToWorld` (`self.Base`)))
  (bind _returnvalue_3 (`|SpawnActorFromClass` "/Game/Blueprints/EnemyFire.EnemyFire_C" (`KismetMathLibrary.MakeTransform` (`KismetMathLibrary.MakeVector` (- (.x (.location _returnvalue_2)) 42.5) (.y (.location _returnvalue_2)) (- (.z (.location _returnvalue_2)) 82.5)) (.rotation _returnvalue_2) (2.0 1.0 2.0)) "Undefined" "OverrideRootScale" null null))
  (set `/Game/Blueprints/EnemyFire.CurDamage` 10 _returnvalue_3)
  (bind _returnvalue_4 (`|SpawnActorFromClass` "/Game/Blueprints/EnemyFire.EnemyFire_C" (`KismetMathLibrary.MakeTransform` (`KismetMathLibrary.MakeVector` (- (.x (.location _returnvalue)) -42.5) (.y (.location _returnvalue)) (- (.z (.location _returnvalue)) 82.5)) (.rotation _returnvalue) (2.0 1.0 2.0)) "Undefined" "OverrideRootScale" null null))
  (set `/Game/Blueprints/EnemyFire.CurDamage` 10 _returnvalue_4))

(fn `UserConstructionScript`
  (`parent.UserConstructionScript`))