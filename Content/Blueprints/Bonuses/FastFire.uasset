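; Fast-fire bonus that temporarily or reversibly speeds up the player ship's weapons, built on a parent bonus class.
; Applying it divides the blaster and strike wave delays by FastRate, and cancelling multiplies them back.
; An IsFasted flag on the ship triggers a cancel before reapplying, so the effect does not stack.
; Both paths stop and reopen fire after changing the delays.
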(event `self.ReceiveBeginPlay`
  (`parent.ReceiveBeginPlay`))

(event `self.ReceiveTick`
  (params (DeltaSeconds :type "Float (single-precision)"))
  (`parent.ReceiveTick` DeltaSeconds))

(event `self.ApplyBonus`
  (bind _playership (`self.PlayerShip`))
  (bind _playership_2 (`self.PlayerShip`))
  (bind _returnvalue (/ 1.0 (`self.FastRate`)))
  (`parent.ApplyBonus`)
  (if (`/Game/Blueprints/PlayerShip.isFasted` _playership_2)
    (`self.CancelBonus`))
  (set `/Game/Blueprints/PlayerShip.isFasted` true _playership_2)
  (set `/Game/Blueprints/PlayerShip.BlasterDelay` (* (`/Game/Blueprints/PlayerShip.BlasterDelay` _playership) _returnvalue) _playership)
  (set `/Game/Blueprints/PlayerShip.StrikeWaveDelay` (* (`/Game/Blueprints/PlayerShip.StrikeWaveDelay` _playership) _returnvalue) _playership)
  (`/Game/Blueprints/PlayerShip.StopFire` _playership)
  (`/Game/Blueprints/PlayerShip.OpenFire` _playership))

(event `self.CancelBonus`
  (bind _fastrate (`self.FastRate`))
  (bind _playership (`self.PlayerShip`))
  (`parent.CancelBonus`)
  (set `/Game/Blueprints/PlayerShip.BlasterDelay` (* (`/Game/Blueprints/PlayerShip.BlasterDelay` _playership) _fastrate) _playership)
  (set `/Game/Blueprints/PlayerShip.StrikeWaveDelay` (* (`/Game/Blueprints/PlayerShip.StrikeWaveDelay` _playership) _fastrate) _playership)
  (`/Game/Blueprints/PlayerShip.StopFire` _playership)
  (`/Game/Blueprints/PlayerShip.OpenFire` _playership)
  (set `/Game/Blueprints/PlayerShip.isFasted` false _playership))

(fn `UserConstructionScript`
  (`parent.UserConstructionScript`))