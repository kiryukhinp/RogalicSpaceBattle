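; PlayerFire is a player projectile that damages enemies it hits.
; Each tick it moves along its local Z axis at Speed, scaled by delta time.
; When its capsule overlaps an Enemy's component named "MainCollsion" (spelled that way), a DoOnce gate lets it apply CurDamage through AddDamage a single time, then it destroys itself.
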(event `self.Capsule.OnComponentBeginOverlap`
  (params (OverlappedComponent :type "PrimitiveComponent Object Reference") (OtherActor :type "Actor Object Reference") (OtherComp :type "PrimitiveComponent Object Reference") (OtherBodyIndex :type Integer) (bFromSweep :type Boolean) (SweepResult :type "HitResult Structure (by ref)"))
  (bind _asenemy (cast `/Game/Blueprints/Enemy` OtherActor))
  (if (`KismetStringLibrary.EqualEqual_StrStr` (`KismetSystemLibrary.GetObjectName` OtherComp) "MainCollsion")
    (`/Engine/EditorBlueprintResources/StandardMacros.DoOnce` false
      (:`Completed`
        (`/Game/Blueprints/Enemy.AddDamage` _asenemy (`self.CurDamage`))
        (`self.K2_DestroyActor`)))))

(event `self.ReceiveTick`
  (params (DeltaSeconds :type "Float (single-precision)"))
  (`self.K2_AddActorLocalOffset` (`KismetMathLibrary.MakeVector` 0.0 0.0 (* DeltaSeconds (`self.speed`)))))

(fn `UserConstructionScript`)