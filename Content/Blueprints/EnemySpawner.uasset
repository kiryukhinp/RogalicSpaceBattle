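; Spawner Blueprint that drops light enemy fighters, rocks and bombs into play at a random X within the side boundary and a set height.
; Two looping timers start on BeginPlay: a slow one for fighters and a fast one for obstacles.
; Each obstacle spawn rolls against BombProbability to pick a scaled-up bomb or a rock.
; The construction script fills ListOfEnemies with random floats keyed by index, which the spawn functions never read.
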(event `self.ReceiveBeginPlay`
  (`|ExecutionSequence`
    (:`then_0`
      (`KismetSystemLibrary.K2_SetTimer` null "SpawnEnemyLight" 10.0 true))
    (:`then_1`
      (`KismetSystemLibrary.K2_SetTimer` null "SpawnObstacle" 0.3 true))))

(fn `SpawnEnemyLight`
  (bind _sideboundary (`self.SideBoundary`))
  (`|SpawnActorFromClass` "/Game/Blueprints/EnemyLightFighter.EnemyLightFighter_C" (`KismetMathLibrary.MakeTransform` (`KismetMathLibrary.MakeVector` (`KismetMathLibrary.RandomFloatInRange` (* _sideboundary -1.0) _sideboundary) 0.0 (`self.SpawnHight`))) "Undefined" "OverrideRootScale" null null)
  (return))

(fn `SpawnObstacle`
  (bind _sideboundary (`self.SideBoundary`))
  (bind _sideboundary_2 (`self.SideBoundary`))
  (if (<= (`KismetMathLibrary.RandomIntegerInRange` 0 100) (`self.BombProbability`))
    (`|SpawnActorFromClass` "/Game/Blueprints/Bomb.Bomb_C" (`KismetMathLibrary.MakeTransform` (`KismetMathLibrary.MakeVector` (`KismetMathLibrary.RandomFloatInRange` (* _sideboundary -1.0) _sideboundary) 1.0 (`self.SpawnHight`)) (struct) (2.0 2.0 2.0)) "Undefined" "OverrideRootScale" null null)
    (else
      (`|SpawnActorFromClass` "/Game/Blueprints/Rock.Rock_C" (`KismetMathLibrary.MakeTransform` (`KismetMathLibrary.MakeVector` (`KismetMathLibrary.RandomFloatInRange` (* _sideboundary_2 -1.0) _sideboundary_2) 0.0 (`self.SpawnHight`))) "Undefined" "OverrideRootScale" null null)))
  (return))

(fn `UserConstructionScript`
  (for _ (range 201)
    (`KismetArrayLibrary.Array_Add` (`self.listOfEnemies`) (make `/Game/Blueprints/EnemyList` null (`KismetMathLibrary.RandomFloatInRange` 0.1 1.0)))))