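; Player-controlled flipbook ship for a shooter on the X/Z plane, with twin blasters, rockets and a StrikeWave attack.
; Construction script loads stats from the ShipStates save, creating it if missing.
; Tick moves the ship within screen bounds, while timers and DoOnce gates pace blaster and StrikeWave fire.
; Finds the Overlay widget to show health, score, ammo, recharge and pause, switching it to game over when death destroys the ship.
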(event `self.ReceiveBeginPlay`
  ;[1 1 1] Spawning
  (`SceneComponent.K2_SetWorldLocation` (`self.Ship`) (0.0 0.0 -350.0) false false)
  (set `self.Current _Health` (`self.Full_Health`))
  (bind _foundwidgets (`WidgetBlueprintLibrary.GetAllWidgetsOfClass` "/Game/UI/Overlay.Overlay_C"))
  (bind _output_get (set `self.Ovrlay reference` (`|GetArrayItem` _foundwidgets)))
  (set `/Game/UI/Overlay.PlayerShipRef` self _output_get)
  (`/Game/UI/Overlay.Update Health` _output_get (`self.Current _Health`) (`self.Full_Health`)))

(event `StikeWaveFromTouch`
  (bind _strikewavedealy (`self.StrikeWaveDealy`))
  (bind (_returnvalue_location _returnvalue_rotation) (`KismetMathLibrary.BreakTransform` (`SceneComponent.K2_GetComponentToWorld` (`self.Ship`))))
  ;[1 1 1] StrikeWave
  (`/Engine/EditorBlueprintResources/StandardMacros.DoOnce` false :!label _label
    (:`Completed`
      (bind _returnvalue (`|SpawnActorFromClass` "/Game/Blueprints/StrikeWave.StrikeWave_C" (`KismetMathLibrary.MakeTransform` _returnvalue_location _returnvalue_rotation (2.0 2.0 2.0)) "Undefined" "OverrideRootScale" null null))
      (set `/Game/Blueprints/StrikeWave.Damage` (`self.StrikeWaveDamage`) _returnvalue)
      (`/Game/UI/Overlay.RechargeWeapon` (`self.Ovrlay reference`) _strikewavedealy)
      (`KismetSystemLibrary.Delay` _strikewavedealy)
      (goto _label :!via `Reset`))))

(event `InputAction|StrikeWave`
  (params (Key :type "Key Structure"))
  ;[1 1 1] StrikeWave
  (:`Pressed`
    (goto _label)))

(event `self.ReceiveTick`
  (params (DeltaSeconds :type "Float (single-precision)"))
  (bind _ship (`self.Ship`))
  (bind _ship_2 (`self.Ship`))
  (bind (_returnvalue_x _returnvalue_y _returnvalue_z) (`KismetMathLibrary.BreakVector` (`SceneComponent.K2_GetComponentLocation` (`self.Ship`))))
  (bind _returnvalue (`KismetMathLibrary.Abs` _returnvalue_z))
  (bind _returnvalue_2 (`KismetMathLibrary.Abs` _returnvalue_x))
  (bind _returnvalue_x_2 (`KismetMathLibrary.BreakVector` (* (+ (* (`SceneComponent.GetUpVector` _ship) (* (`self.Max_Sped`) (`self.GetInputAxisValue`))) (* (`SceneComponent.GetForwardVector` _ship) (* (`self.GetInputAxisValue`) (`self.Max_Sped`)))) DeltaSeconds)))
  ;[1 1 1] Movement execute
  (if (and (<= _returnvalue_2 600.0) (<= _returnvalue 400.0))
    (`SceneComponent.K2_AddLocalOffset` _ship_2 (`KismetMathLibrary.MakeVector` _returnvalue_x_2) true false)
    (else
      (`SceneComponent.K2_AddLocalOffset` _ship_2 (`KismetMathLibrary.MakeVector` (* (/ _returnvalue_2 _returnvalue_x) -1.0) 0.0 (* (/ _returnvalue_z _returnvalue) -1.0)) false false))))

(event `InputAction|Fire`
  (params (Key :type "Key Structure"))
  ;[1 1 1] Fire action control
  (:`Pressed`
    (`/Engine/EditorBlueprintResources/StandardMacros.DoOnce` false :!label _label_2
      (:`Completed`
        (`PaperFlipbookComponent.SetFlipbook` (`self.Ship`) "/Game/Sprites/Player_SS/SS_Fire.SS_Fire")
        (`self.OpenFire`)
        (`KismetSystemLibrary.Delay` (`self.BlasterDelay`))
        (goto _label_2 :!via `Reset`))))
  (:`Released`
    (`PaperFlipbookComponent.SetFlipbook` (`self.Ship`) "/Game/Sprites/Player_SS/Base_SS_anim.Base_SS_anim")
    (`self.StopFire`)))

(event `StopFire`
  ;[1 1 1] Open blaster fire
  (`KismetSystemLibrary.K2_PauseTimerHandle` (stale `OpenFire` _returnvalue)))

(event `OpenFire`
  ;[1 1 1] Open blaster fire
  (`self.Fire`)
  (bind _returnvalue (`KismetSystemLibrary.K2_SetTimer` null "Fire" (`self.BlasterDelay`) true)))

(event `LaunchRocketByTouch`
  ;[1 1 1] RocketStrike
  (if (> (`self.RocketNum`) 0) :!label _label_3
    (`self.LaunchRocket`)
    (bind _output_get (set `self.RocketNum` (- (`self.RocketNum`) 1)))
    (`TextBlock.SetText` (`/Game/UI/Overlay.TextBlock_3` (`self.Ovrlay reference`)) (`KismetTextLibrary.Conv_IntToText` _output_get))))

(event `InputAction|Rocket`
  (params (Key :type "Key Structure"))
  ;[1 1 1] RocketStrike
  (:`Pressed`
    (goto _label_3)))

(event `AddDmamge`
  (params (Damage :type Integer))
  (bind _ovrlay_reference (`self.Ovrlay reference`))
  ;[1 1 1] Add damage to player
  (set `self.Current _Health` (- (`self.Current _Health`) Damage))
  (`/Game/UI/Overlay.Update Health` (`self.Ovrlay reference`) (`self.Current _Health`) (`self.Full_Health`))
  (if (<= (`self.Current _Health`) 0)
    (set `self.IsGameOver` true)
    (`|SpawnActorFromClass` "/Game/Blueprints/Blow_Up.Blow_Up_C" (`SceneComponent.K2_GetComponentToWorld` (`self.Ship`)) "Undefined" "OverrideRootScale" null null)
    (`WidgetSwitcher.SetActiveWidgetIndex` (`/Game/UI/Overlay.WidgetSwitcher_0` _ovrlay_reference) 1)
    (`TextBlock.SetText` (`/Game/UI/Overlay.TextBlock_120` _ovrlay_reference) (`TextBlock.GetText` (`/Game/UI/Overlay.TextBlock_61` _ovrlay_reference)))
    (`self.K2_DestroyActor`)))

(event `InputAction|Pause` :paused true
  (params (Key :type "Key Structure"))
  (bind _widgetswitcher_0 (`/Game/UI/Overlay.WidgetSwitcher_0` (`self.Ovrlay reference`)))
  ;[1 1 1] Set Pause
  (:`Pressed`
    (if (not (`self.IsGameOver`))
      (`/Engine/EditorBlueprintResources/StandardMacros.FlipFlop`
        (:`A`
          (`GameplayStatics.SetGamePaused` true)
          (`WidgetSwitcher.SetActiveWidgetIndex` _widgetswitcher_0 2))
        (:`B`
          (`GameplayStatics.SetGamePaused` false)
          (`WidgetSwitcher.SetActiveWidgetIndex` _widgetswitcher_0 0))))))

(fn `AddCoins`
  (params (Add :type Integer))
  (`/Game/UI/Overlay.Update Score` (`self.Ovrlay reference`) Add))

(fn `Fire`
  (bind _returnvalue (`SceneComponent.K2_GetComponentToWorld` (`self.Ship`)))
  (bind _returnvalue_2 (`SceneComponent.K2_GetComponentToWorld` (`self.Ship`)))
  (bind _returnvalue_3 (`|SpawnActorFromClass` "/Game/Blueprints/Fire.Fire_C" (`KismetMathLibrary.MakeTransform` (`KismetMathLibrary.MakeVector` (+ (.x (.location _returnvalue_2)) 33.0) (.y (.location _returnvalue_2)) (+ (.z (.location _returnvalue_2)) 50.0)) (struct) (2.0 1.0 2.0)) "Undefined" "OverrideRootScale" null null))
  (set `/Game/Blueprints/Fire.CurDamage` (`self.BlasterDamage`) _returnvalue_3)
  (bind _returnvalue_4 (`|SpawnActorFromClass` "/Game/Blueprints/Fire.Fire_C" (`KismetMathLibrary.MakeTransform` (`KismetMathLibrary.MakeVector` (+ (.x (.location _returnvalue)) -33.0) (.y (.location _returnvalue)) (+ (.z (.location _returnvalue)) 50.0)) (struct) (2.0 1.0 2.0)) "Undefined" "OverrideRootScale" null null))
  (set `/Game/Blueprints/Fire.CurDamage` (`self.BlasterDamage`) _returnvalue_4))

(fn `LaunchRocket`
  (bind _returnvalue (`|SpawnActorFromClass` "/Game/Blueprints/Rocket.Rocket_C" (`KismetMathLibrary.MakeTransform` (`SceneComponent.K2_GetComponentLocation` (`self.Ship`)) (struct) (0.25 1.0 0.25)) "Undefined" "OverrideRootScale" null null))
  (set `/Game/Blueprints/Rocket.RocketDamge` (`self.RocketDamage`) _returnvalue))

(fn `UserConstructionScript`
  (bind _returnvalue (`GameplayStatics.DoesSaveGameExist` (`self.DefaultGameSlot`)))
  (if (not _returnvalue)
    (bind _returnvalue_2 (`GameplayStatics.CreateSaveGameObject` "/Game/Saves/ShipStates.ShipStates_C"))
    (bind _output_get (set `self.SaveGame` _returnvalue_2))
    (`GameplayStatics.SaveGameToSlot` _output_get (`self.DefaultGameSlot`)))
  (bind _returnvalue_3 (`GameplayStatics.LoadGameFromSlot` (`self.DefaultGameSlot`)))
  (bind _output_get_2 (set `self.SaveGame` _returnvalue_3))
  (bind _asship_states (cast `/Game/Saves/ShipStates` _output_get_2))
  (set `self.Max_Sped` (`/Game/Saves/ShipStates.Speed` _asship_states))
  (set `self.BlasterDamage` (`/Game/Saves/ShipStates.BlasterDamage` _asship_states))
  (set `self.BlasterDelay` (`/Game/Saves/ShipStates.BlasterDelay` _asship_states))
  (set `self.Full_Health` (`/Game/Saves/ShipStates.Health` _asship_states))
  (set `self.StrikeWaveDamage` (`/Game/Saves/ShipStates.StrikeWaveDamage` _asship_states))
  (set `self.StrikeWaveDealy` (`/Game/Saves/ShipStates.StrikeWaveDelay` _asship_states))
  (set `self.RocketDamage` (`/Game/Saves/ShipStates.RocketDamge` _asship_states))
  (set `self.RocketNum` (`/Game/Saves/ShipStates.RocketNum` _asship_states)))