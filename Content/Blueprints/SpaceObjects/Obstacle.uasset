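; Obstacle is a space object Blueprint that moves steadily along world negative Z.
; Each Tick offsets the actor by Speed scaled by delta time, using teleport and no sweep, so movement is frame-rate independent.
; BeginPlay, OnHit damage handling and construction only forward to the parent class, which supplies all other behavior.
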(event `self.ReceiveBeginPlay`
  (`parent.ReceiveBeginPlay`))

(event `self.ReceiveTick`
  (params (DeltaSeconds :type "Float (single-precision)"))
  (`parent.ReceiveTick` DeltaSeconds)
  (`self.K2_AddActorWorldOffset` (`KismetMathLibrary.MakeVector` 0.0 0.0 (/ (* (`self.Speed`) -1.0) (/ 1.0 DeltaSeconds))) false true))

(event `self.OnHit`
  (params (Damage :type Integer))
  (`parent.OnHit` Damage))

(fn `UserConstructionScript`
  (`parent.UserConstructionScript`))