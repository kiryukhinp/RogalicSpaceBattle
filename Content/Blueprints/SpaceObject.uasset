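; SpaceObject is an actor for space objects that damage the player ship on contact and can drop coins.
; When its Sphere overlaps a PlayerShip, it applies bump damage and calls Blow.
; Blow optionally spawns a Blow_Up effect scaled by blow radius, calls Drop for a probability-based Coin spawn carrying a set value, then destroys the actor.
; OnHit takes damage but is an empty stub here.
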(event `self.Sphere.OnComponentBeginOverlap`
  (params (OverlappedComponent :type "PrimitiveComponent Object Reference") (OtherActor :type "Actor Object Reference") (OtherComp :type "PrimitiveComponent Object Reference") (OtherBodyIndex :type Integer) (bFromSweep :type Boolean) (SweepResult :type "HitResult Structure (by ref)"))
  (bind _asplayer_ship (cast `/Game/Blueprints/PlayerShip` OtherActor))
  (`/Game/Blueprints/PlayerShip.AddDmamge` _asplayer_ship (`self.BumpDamage`))
  (`self.Blow`))

(fn `Blow`
  (bind _returnvalue (`self.GetTransform`))
  (if (`self.PlayBlowAnim`)
    (`|SpawnActorFromClass` "/Game/Blueprints/Blow_Up.Blow_Up_C" (`KismetMathLibrary.MakeTransform` (`KismetMathLibrary.MakeVector` (.x (.location _returnvalue)) 1.0 (.z (.location _returnvalue))) (.rotation _returnvalue) (`KismetMathLibrary.Conv_DoubleToVector` (`self.BlowRadius`))) "Undefined" "OverrideRootScale" null null))
  (`self.Drop`)
  (`self.K2_DestroyActor`))

(fn `Drop`
  (bind (_returnvalue_location _returnvalue_rotation) (`KismetMathLibrary.BreakTransform` (`SceneComponent.K2_GetComponentToWorld` (`self.PaperFlipbook`))))
  (if (<= (`KismetMathLibrary.RandomIntegerInRange` 0 100) (`self.CoinProbability`))
    (`|SpawnActorFromClass` "/Game/Blueprints/Coin.Coin_C" (`KismetMathLibrary.MakeTransform` _returnvalue_location _returnvalue_rotation (2.5 1.0 2.5)) "Undefined" "OverrideRootScale" null (`self.CoinValue`) null)
    (return)))

(fn `OnHit`
  (params (Damage :type Integer))
  (return))

(fn `UserConstructionScript`)