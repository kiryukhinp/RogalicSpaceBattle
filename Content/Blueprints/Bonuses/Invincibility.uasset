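; Invincibility bonus Blueprint that makes the player ship invincible and restores it to full health.
; It extends a parent bonus class through ApplyBonus and CancelBonus, calling the parent version of each first.
; Applying it to an already invincible ship runs CancelBonus before setting the flag again and refilling health.
; CancelBonus clears the ship's invincibility flag, and this Blueprint adds no timing logic of its own.
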(event `self.ReceiveBeginPlay`
  (`parent.ReceiveBeginPlay`))

(event `self.ReceiveTick`
  (params (DeltaSeconds :type "Float (single-precision)"))
  (`parent.ReceiveTick` DeltaSeconds))

(event `self.ApplyBonus`
  (bind _playership (`self.PlayerShip`))
  (bind _playership_2 (`self.PlayerShip`))
  (`parent.ApplyBonus`)
  (if (`/Game/Blueprints/PlayerShip.isInvincible` _playership_2)
    (`self.CancelBonus`))
  (set `/Game/Blueprints/PlayerShip.isInvincible` true _playership_2)
  (set `/Game/Blueprints/PlayerShip.Current _Health` (`/Game/Blueprints/PlayerShip.Full_Health` _playership) _playership))

(event `self.CancelBonus`
  (`parent.CancelBonus`)
  (set `/Game/Blueprints/PlayerShip.isInvincible` false (`self.PlayerShip`)))

(fn `UserConstructionScript`
  (`parent.UserConstructionScript`))