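; Enemy space object that moves toward the player along its local Z axis at Speed and can be destroyed by damage.
; On hit it subtracts damage from its health; at zero it adds a point on the Overlay widget found at BeginPlay and calls Blow.
; Non-lethal hits reveal the health bar component once, update its fill from the health ratio and print that ratio.
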(event `self.ReceiveBeginPlay`
  ;[1 1 1] Set widget links
  (bind _foundwidgets (`WidgetBlueprintLibrary.GetAllWidgetsOfClass` "/Game/UI/Overlay.Overlay_C"))
  (set `self.Overlay_ref` (`|GetArrayItem` _foundwidgets))
  (set `self.CurHealth` (`self.DefaultHealth`)))

(event `self.OnHit`
  (params (Damage :type Integer))
  (bind _returnvalue (/ (`KismetMathLibrary.Conv_IntToDouble` (`self.CurHealth`)) (`KismetMathLibrary.Conv_IntToDouble` (`self.DefaultHealth`))))
  ;[1 1 1] Add damage
  (`parent.OnHit` Damage)
  (bind _output_get (set `self.CurHealth` (- (`self.CurHealth`) Damage)))
  (if (<= _output_get 0)
    (`/Game/UI/Overlay.Update Score` (`self.Overlay_ref`) 1)
    (`self.Blow`)
    (else
      (`|ExecutionSequence`
        (:`then_0`
          (`/Engine/EditorBlueprintResources/StandardMacros.DoOnce` false
            (:`Completed`
              (`SceneComponent.SetHiddenInGame` (`self.HealthBar`) false false))))
        (:`then_1`
          (bind _asenemy_health_bar (cast `/Game/UI/EnemyHealthBar` (`WidgetComponent.GetUserWidgetObject` (`self.HealthBar`))))
          (`ProgressBar.SetPercent` (`/Game/UI/EnemyHealthBar.Health` _asenemy_health_bar) _returnvalue)
          (`KismetSystemLibrary.PrintString` (`KismetStringLibrary.Conv_DoubleToString` _returnvalue)))))))

(event `self.ReceiveTick`
  (params (DeltaSeconds :type "Float (single-precision)"))
  ;[1 1 1] Motion to player
  (`parent.ReceiveTick` DeltaSeconds)
  (`self.K2_AddActorLocalOffset` (`KismetMathLibrary.MakeVector` 0.0 0.0 (* (`self.Speed`) DeltaSeconds))))

(fn `UserConstructionScript`)