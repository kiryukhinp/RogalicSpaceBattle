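; Base space object that damages the player ship on overlap, then blows up and drops loot.
; Blow optionally spawns an explosion scaled by BlowRadius, calls Drop and destroys the actor.
; Drop independently rolls for a coin carrying CoinValue and for a bonus whose class comes from a random BonusesTable row.
; OnHit takes a Damage input but is an empty stub here.
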(event `self.ReceiveActorBeginOverlap`
  (params (OtherActor :type "Actor Object Reference"))
  (`/Engine/EditorBlueprintResources/StandardMacros.IsValid` OtherActor
    (:`Is Valid`
      (bind _asplayer_ship (cast `/Game/Blueprints/PlayerShip` OtherActor))
      (`/Game/Blueprints/PlayerShip.AddDmamge` _asplayer_ship (`self.BumpDamage`))
      (`self.Blow`))))

(fn `Blow`
  (bind _returnvalue (`self.GetTransform`))
  (if (`self.PlayBlowAnim`)
    (`|SpawnActorFromClass` "/Game/Blueprints/Blow_Up.Blow_Up_C" (`KismetMathLibrary.MakeTransform` (`KismetMathLibrary.MakeVector` (.x (.location _returnvalue)) 1.0 (.z (.location _returnvalue))) (.rotation _returnvalue) (`KismetMathLibrary.Conv_DoubleToVector` (`self.BlowRadius`))) "Undefined" "OverrideRootScale" null null))
  (`self.Drop`)
  (`self.K2_DestroyActor`))

(fn `Drop`
  (bind _bonusestable (`self.BonusesTable`))
  (bind (_returnvalue_location _returnvalue_rotation) (`KismetMathLibrary.BreakTransform` (`SceneComponent.K2_GetComponentToWorld` (`self.PaperFlipbook`))))
  (bind (_returnvalue_location_2 _returnvalue_rotation_2) (`KismetMathLibrary.BreakTransform` (`SceneComponent.K2_GetComponentToWorld` (`self.PaperFlipbook`))))
  (`|ExecutionSequence`
    (:`then_0`
      (if (<= (`KismetMathLibrary.RandomIntegerInRange` 0 100) (`self.CoinProbability`))
        (`|SpawnActorFromClass` "/Game/Blueprints/Coin.Coin_C" (`KismetMathLibrary.MakeTransform` _returnvalue_location _returnvalue_rotation (2.5 1.0 2.5)) "Undefined" "OverrideRootScale" null (`self.CoinValue`) null)))
    (:`then_1`
      (if (<= (`KismetMathLibrary.RandomIntegerInRange` 0 100) (`self.BonusProbability`))
        (bind _outrownames (`DataTableFunctionLibrary.GetDataTableRowNames` _bonusestable))
        (bind _returnvalue (`|GetDataTableRow` _bonusestable (`|GetArrayItem` _outrownames (`KismetMathLibrary.RandomInteger` (`KismetArrayLibrary.Array_Length` _outrownames))))
          (:`then`
            (`|SpawnActorFromClass` (`.Bonus_2_6D255D9F435551E23CEA7D84EE5A6923` (break `/Game/Blueprints/Bonuses/Bonuses` _returnvalue)) (`KismetMathLibrary.MakeTransform` _returnvalue_location_2 _returnvalue_rotation_2 (2.5 1.0 2.5)) "Undefined" "OverrideRootScale" null null)))))
    (:`then_2`
      (return))))

(fn `OnHit`
  (params (Damage :type Integer))
  (return))

(fn `UserConstructionScript`)