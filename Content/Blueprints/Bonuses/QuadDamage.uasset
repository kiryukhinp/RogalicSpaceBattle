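; Quad Damage bonus that quadruples the player ship's blaster, rocket and strike wave damage.
; It extends a parent bonus class through ApplyBonus and CancelBonus, calling the parent version first in each.
; ApplyBonus sets the ship's IsQuaded flag, first calling CancelBonus if already set so the multiplier does not stack.
; CancelBonus divides the damage values back and clears the flag.
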(event `self.ReceiveBeginPlay`
  (`parent.ReceiveBeginPlay`))

(event `self.ApplyBonus`
  (bind _playership (`self.PlayerShip`))
  (bind _playership_2 (`self.PlayerShip`))
  (`parent.ApplyBonus`)
  (if (`/Game/Blueprints/PlayerShip.isQuaded` _playership_2)
    (`self.CancelBonus`))
  (set `/Game/Blueprints/PlayerShip.isQuaded` true _playership_2)
  (set `/Game/Blueprints/PlayerShip.BlasterDamage` (* (`/Game/Blueprints/PlayerShip.BlasterDamage` _playership) 4) _playership)
  (set `/Game/Blueprints/PlayerShip.RocketDamage` (* (`/Game/Blueprints/PlayerShip.RocketDamage` _playership) 4) _playership)
  (set `/Game/Blueprints/PlayerShip.StrikeWaveDamage` (* (`/Game/Blueprints/PlayerShip.StrikeWaveDamage` _playership) 4) _playership))

(event `self.CancelBonus`
  (bind _playership (`self.PlayerShip`))
  (`parent.CancelBonus`)
  (set `/Game/Blueprints/PlayerShip.BlasterDamage` (/ (`/Game/Blueprints/PlayerShip.BlasterDamage` _playership) 4) _playership)
  (set `/Game/Blueprints/PlayerShip.RocketDamage` (/ (`/Game/Blueprints/PlayerShip.RocketDamage` _playership) 4) _playership)
  (set `/Game/Blueprints/PlayerShip.StrikeWaveDamage` (/ (`/Game/Blueprints/PlayerShip.StrikeWaveDamage` _playership) 4) _playership)
  (set `/Game/Blueprints/PlayerShip.isQuaded` false _playership))

(fn `UserConstructionScript`
  (`parent.UserConstructionScript`))