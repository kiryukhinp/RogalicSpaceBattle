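; Asteroid actor that randomizes its horizontal placement when spawned.
; On BeginPlay it calls the parent, then shifts its Base component along world X by a random offset within a fixed symmetric range, keeping Y and Z.
; Overlap and Tick events are disabled stubs, and the construction script only calls the parent, so any other behavior comes from outside this graph.
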(event `self.ReceiveBeginPlay`
  (bind (_returnvalue_x _returnvalue_y _returnvalue_z) (`KismetMathLibrary.BreakVector` (`SceneComponent.K2_GetComponentLocation` (`self.Base`))))
  (`parent.ReceiveBeginPlay`)
  (`SceneComponent.K2_SetWorldLocation` (`self.Base`) (`KismetMathLibrary.MakeVector` (+ _returnvalue_x (`KismetMathLibrary.RandomFloatInRange` -300.0 300.0)) _returnvalue_y _returnvalue_z) false false))

(fn `UserConstructionScript`
  (`parent.UserConstructionScript`))