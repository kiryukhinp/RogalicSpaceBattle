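; Enemy spawner actor with two spawn paths: random asteroids and an ordered enemy list.
; BeginPlay starts a looping timer for randomly placed and scaled asteroid-style spawns, then pauses it after a zero-length delay.
; It then spawns from ListOfEnemies at the spawner's XY with fixed height and advances Index, with a Gate wired back to that spawn.
; Overlap, Tick and construction logic are empty.
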(event `self.ReceiveBeginPlay`
  (bind _returnvalue (`self.GetTransform`))
  (bind _returnvalue_2 (`KismetSystemLibrary.K2_SetTimer` null "Spawn_Asteroid" 0.5 true))
  (`KismetSystemLibrary.Delay` 0.0)
  (`KismetSystemLibrary.K2_PauseTimerHandle` _returnvalue_2)
  (`|SpawnActorFromClass` (`|GetArrayItem` (`self.listOfEnemies`) (`self.Index`)) (`KismetMathLibrary.MakeTransform` (`KismetMathLibrary.MakeVector` (.x (.location _returnvalue)) (.y (.location _returnvalue)) 300.0) (struct) (0.5 0.5 0.5)) "Undefined" "OverrideRootScale" null null :!label _label)
  (`/Engine/EditorBlueprintResources/StandardMacros.IncrementInt` (`self.Index`)
    (:`  `
      (`/Engine/EditorBlueprintResources/StandardMacros.Gate` true
        (:`Exit`
          (goto _label))))))

(fn `Spawn_Asteroid`
  (bind (_returnvalue_x _returnvalue_y _returnvalue_z) (`KismetMathLibrary.BreakVector` (`self.K2_GetActorLocation`)))
  (bind _returnvalue (`KismetMathLibrary.RandomFloatInRange` 0.3 0.8))
  (`|SpawnActorFromClass` "/Game/Blueprints/Enemy.Enemy_C" (`KismetMathLibrary.MakeTransform` (`KismetMathLibrary.MakeVector` (`KismetMathLibrary.RandomFloatInRange` -600.0 600.0) _returnvalue_y _returnvalue_z) (struct :`Pitch` -180.0) (`KismetMathLibrary.MakeVector` _returnvalue 0.5 _returnvalue)) "Undefined" "OverrideRootScale" null null))

(fn `UserConstructionScript`)