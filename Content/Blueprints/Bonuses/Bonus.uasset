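; Base pickup for timed bonuses that drift down along world Z until the player ship collects them.
; BeginPlay caches the player ship, and Tick moves the actor by Speed scaled with delta time.
; On overlap with the ship, ApplyBonus hides the pickup and disables collision and tick, then after LifeTime CancelBonus runs and the actor is destroyed.
; CancelBonus is empty, and ApplyBonus grants no effect itself.
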(event `self.ReceiveBeginPlay`
  (bind _asplayer_ship (cast `/Game/Blueprints/PlayerShip` (`GameplayStatics.GetPlayerPawn` 0)))
  (set `self.PlayerShip` _asplayer_ship))

(event `self.ReceiveActorBeginOverlap`
  (params (OtherActor :type "Actor Object Reference"))
  (cast `/Game/Blueprints/PlayerShip` OtherActor)
  (`self.ApplyBonus`)
  (`KismetSystemLibrary.Delay` (`self.LifeTime`))
  (`self.CancelBonus`)
  (`self.K2_DestroyActor`))

(event `self.ReceiveTick`
  (params (DeltaSeconds :type "Float (single-precision)"))
  (`self.K2_AddActorWorldOffset` (`KismetMathLibrary.MakeVector` 0.0 0.0 (/ (* (`self.Speed`) -1.0) (/ 1.0 DeltaSeconds))) false true))

(fn `ApplyBonus`
  (`self.SetActorEnableCollision` false)
  (`self.SetActorTickEnabled` false)
  (`self.SetActorHiddenInGame` true)
  (return))

(fn `CancelBonus`
  (return))

(fn `UserConstructionScript`)