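; Homing rocket actor that locks onto a random Enemy on spawn and damages enemies it hits.
; Each tick it moves along its up vector, then pitches by the full angle to the target (arccosine of a dot product), signed by comparing X components.
; With no valid target it flies straight.
; Overlapping an Enemy's "MainCollsion" component applies damage, spawns a Blow_Up actor and destroys the rocket.
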(event `self.ReceiveBeginPlay`
  (bind _outactors (`GameplayStatics.GetAllActorsOfClass` "/Game/Blueprints/Enemy.Enemy_C"))
  (set `self.Target` (`|GetArrayItem` _outactors (`KismetMathLibrary.RandomIntegerInRange` 0 (- (`KismetArrayLibrary.Array_Length` _outactors) 1))))
  (`KismetSystemLibrary.Delay` 0.5))

(event `self.ReceiveTick`
  (params (DeltaSeconds :type "Float (single-precision)"))
  (`self.K2_AddActorWorldOffset` (* (`self.GetActorUpVector`) (* DeltaSeconds (`self.Speed`))))
  (`self.RotateToTarget`))

(event `self.Capsule.OnComponentBeginOverlap`
  (params (OverlappedComponent :type "PrimitiveComponent Object Reference") (OtherActor :type "Actor Object Reference") (OtherComp :type "PrimitiveComponent Object Reference") (OtherBodyIndex :type Integer) (bFromSweep :type Boolean) (SweepResult :type "HitResult Structure (by ref)"))
  (bind _asenemy (cast `/Game/Blueprints/Enemy` OtherActor))
  (if (`KismetStringLibrary.EqualEqual_StrStr` (`KismetSystemLibrary.GetObjectName` OtherComp) "MainCollsion")
    (`/Game/Blueprints/Enemy.AddDamage` _asenemy (`self.RocketDamge`))
    (`self.BlowUp`)))

(fn `BlowUp`
  (`|SpawnActorFromClass` "/Game/Blueprints/Blow_Up.Blow_Up_C" (`KismetMathLibrary.MakeTransform` (`SceneComponent.K2_GetComponentLocation` (`self.Box`)) (struct) (0.5 0.5 0.5)) "Undefined" "OverrideRootScale" null null)
  (`self.K2_DestroyActor`))

(fn `RotateToTarget`
  (bind (_returnvalue_x _returnvalue_y _returnvalue_z) (`KismetMathLibrary.BreakVector` (`self.GetActorUpVector`)))
  (bind _target (`self.Target`))
  (bind (_returnvalue_x_2 _returnvalue_y_2 _returnvalue_z_2) (`KismetMathLibrary.BreakVector` (`KismetMathLibrary.Normal` (- (`self.K2_GetActorLocation` _target) (`self.K2_GetActorLocation`)))))
  (bind _returnvalue (`KismetMathLibrary.DegAcos` (`KismetMathLibrary.Dot_VectorVector` (`KismetMathLibrary.MakeVector` _returnvalue_x_2 _returnvalue_y_2 _returnvalue_z_2) (`KismetMathLibrary.MakeVector` _returnvalue_x _returnvalue_y _returnvalue_z))))
  (`/Engine/EditorBlueprintResources/StandardMacros.IsValid` _target
    (:`Is Valid`
      (if (> _returnvalue_x _returnvalue_x_2)
        (`self.K2_AddActorLocalRotation` (`KismetMathLibrary.MakeRotator` 0.0 _returnvalue))
        (else
          (`self.K2_AddActorLocalRotation` (`KismetMathLibrary.MakeRotator` 0.0 (* _returnvalue -1.0))))))))

(fn `UserConstructionScript`)